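; BP_DamageIndicator is a short-lived floating damage indicator that displays a hit value through its WBP_HitDamage widget.
; On BeginPlay it copies Damage from the first BP_ThirdPersonCharacter found in the world into the widget.
; The DamageAnimation timeline then lerps the actor from its spawn location up and slightly sideways along a fixed world offset, and destroys it on finish.
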(event EventBeginPlay
  (bind _returnvalue (Actor|GetActorOfClass "/Game/ThirdPerson/Blueprints/BP_ThirdPersonCharacter.BP_ThirdPersonCharacter_C"))
  (bind _aswbp_hit_damage (Utilities|Casting|CastToWBP_HitDamage (UserInterface|GetWidget (Variables|Default|GetWidget))))
  (Variables|/Game/UI/HUD/WBP_HitDamage.WBP_HitDamage_C|SetDamage _aswbp_hit_damage (Variables|/Game/ThirdPerson/Blueprints/BP_ThirdPersonCharacter.BP_ThirdPersonCharacter_C|GetDamage _returnvalue))
  (bind _output_get (Variables|Default|SetInitial%20Location (Transformation|GetActorLocation)))
  (Variables|Default|SetEnd%20Location (+ _output_get "-25.000000,-25.000000,100.000000"))
  (bind _newtrack_0 (Timeline|Damage%20Animation Play)
    (:Update
      (Transformation|SetActorLocation (Math|Vector|Lerp(Vector) (Variables|Default|GetInitial%20Location) (Variables|Default|GetEnd%20Location) _newtrack_0) false false))
    (:Finished
      (Actor|DestroyActor))))

(fn ConstructionScript)