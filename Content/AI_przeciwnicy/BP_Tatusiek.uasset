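; BP_Tatusiek is a revolver-wielding AI enemy that shoots at the player and ragdolls on death.
; AnyDamage lowers HEALTH; at zero it sets IsDead, disables movement and capsule collision, and hides the health bar.
; Fire line-traces from the muzzle toward the player, applies damage and spawns effects, with a DoOnce and random delay as cooldown.
; Aim sets IsAiming, while Tick updates the health bar widget and turns it toward the camera.
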(event EventTick
  (params (DeltaSeconds :type Float%20%28single-precision%29))
  ;[0.7679 1 0.7112] helth bar AI
  (bind _ashealth_bar_ai (Utilities|Casting|CastToHealth_bar_AI (UserInterface|GetWidget (Variables|Default|GetHealth_Bar_AI))))
  (Progress|SetPercent (Variables|/Game/UI/HUD/Health_bar_AI.Health_bar_AI_C|GetHelth_Bar_AI _ashealth_bar_ai) (/ (Variables|Default|GetHEALTH) 25.0))
  (Transformation|SetWorldRotation (Variables|Default|GetHealth_Bar_AI) (Math|Rotator|FindLookatRotation (Transformation|GetActorLocation) (Transformation|GetActorLocation (Game|GetPlayerCameraManager 0))) false false))

(event Game|Damage|EventAnyDamage
  (params (Damage :type Float%20%28single-precision%29) (DamageType :type Damage%20Type%20Object%20Reference) (InstigatedBy :type Controller%20Object%20Reference) (DamageCauser :type Actor%20Object%20Reference))
  ;[0.5551 1 0.6452] HEALTH SYSTEM
  (Variables|Default|SetHEALTH (- (Variables|Default|GetHEALTH) Damage))
  (if (<= (Variables|Default|GetHEALTH) 0.0)
    (Development|PrintString "CIUPAZECKA")
    (Physics|SetSimulatePhysics (Variables|Character|GetMesh) true)
    (Pawn|Components|CharacterMovement|SetMovementMode (Variables|Character|GetCharacterMovement) "MOVE_None" 0)
    (Variables|Default|SetisDead? true)
    (Collision|SetCollisionEnabled (Variables|Collision|GetCapsuleComponent) "NoCollision")
    (Variables|Default|SetisDead? true)
    (Rendering|SetVisibility (Variables|Default|GetHealth_Bar_AI) false false)
    (else
      (Development|PrintString "ŁOSCYOPECEK"))))

(event EventFire
  (bind _rewolwer_ai (Variables|Default|GetRewolwer_AI))
  (bind _returnvalue (Transformation|GetSocketTransform _rewolwer_ai "b_gun_muzzleflash" "RTS_World"))
  ;[1 1 1] Fire
  (if (not (Variables|Default|GetisDead?))
    (Utilities|FlowControl|DoOnce false :!label _label
      (:Completed
        (Utilities|FlowControl|Sequence
          (:then_0
            (Effects|SpawnEmitterAttached "/Game/VFX/Inventory/Props/FX/P_Pistol_MuzzleFlash_01.P_Pistol_MuzzleFlash_01" (Variables|Default|GetRewolwer_AI) "b_gun_muzzleflash" (.location _returnvalue) (Transformation|GetWorldRotation (Variables|Character|GetMesh)) "0.250000,0.250000,0.250000" "KeepWorldPosition" true "AutoRelease")
            (Audio|PlaySoundatLocation "/Game/DZWIEK/MS_Pistolero_Fire.MS_Pistolero_Fire" (Transformation|GetActorLocation) "0, 0, 0" 0.15 1.0 0.0 0 0 0 0)
            (bind _outhit (Collision|LineTraceByChannel (.location _returnvalue) (+ (* (Math|Vector|GetForwardVector (Math|Rotator|FindLookatRotation (.location (Transformation|GetSocketTransform (Variables|Default|GetRewolwer_AI) "b_gun_muzzleflash" "RTS_World")) (Transformation|GetActorLocation (Game|GetPlayerCharacter 0)))) 3e+03) (.location _returnvalue)) "TraceTypeQuery1" false 0 "ForDuration"))
            (if true
              (Game|Damage|ApplyDamage (.HitActor (Collision|BreakHitResult _outhit)) 5.0 0 0)
              (Rendering|Decal|SpawnDecalatLocation "/Game/VFX/Inventory/Props/FX/bullet_whole.bullet_whole" (Math|Conversions|ToVector(Float) (Math|Random|RandomIntegerinRange 5 6)) (.ImpactPoint (Collision|BreakHitResult _outhit)) (Math|Rotator|MakeRotfromX (.Normal (Collision|BreakHitResult _outhit))) 8.0)
              (Audio|PlaySoundatLocation "/Game/DZWIEK/MS_bullet.MS_bullet" (.ImpactPoint (Collision|BreakHitResult _outhit)) "0, 0, 0" 0.2 1.0 0.0 0 0 0 0)))
          (:then_1
            (Utilities|FlowControl|Delay (Math|Random|RandomFloatinRange 0.5 3.0))
            (goto _label Reset)))))))

(event EventAim
  (params (Aim? :type Boolean))
  (Variables|Default|SetisAiming Aim?))

(fn ConstructionScript)