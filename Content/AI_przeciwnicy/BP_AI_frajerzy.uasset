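; AI controller for BP_Enemy pawns that runs the BT_frajerzy behavior tree and reacts to perceiving the player.
; On BeginPlay it caches the controlled enemy and writes its movement mode to the blackboard.
; When perception senses the player, the enemy starts aiming and the blackboard receives the player and a new AI state.
; When the player is lost, it stores the player's current location as last known and switches the AI state again.
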(event OnTargetPerceptionUpdated(AIPerception)
  (params (Actor :type Actor%20Object%20Reference) (Stimulus :type AI%20Stimulus%20Structure))
  (Variables|Default|SetStimulus Stimulus)
  (if (.bSuccessfullySensed (Utilities|Struct|BreakAIStimulus Stimulus))
    (if (== Actor (Game|GetPlayerCharacter 0))
      (Default|Aim (Variables|Default|GetEnemy) true)
      (AI|Components|Blackboard|SetValueasEnum (AI|GetBlackboard 0) (Utilities|Name|MakeLiteralName "AIState") (Utilities|Enum|LiteralenumE_EnemyBheaviorStates "NewEnumerator2"))
      (AI|Components|Blackboard|SetValueasObject (AI|GetBlackboard 0) (Utilities|Name|MakeLiteralName "Player") (Game|GetPlayerCharacter 0)))
    (elif (== Actor (Game|GetPlayerCharacter 0))
      (Development|PrintString "Lost Player" true true "(R=1.000000,G=0.922610,B=0.000000,A=1.000000)")
      (AI|Components|Blackboard|SetValueasVector (AI|GetBlackboard 0) (Utilities|Name|MakeLiteralName "LastKnownPlayerLocation") (Transformation|GetActorLocation (Game|GetPlayerCharacter 0)))
      (AI|Components|Blackboard|SetValueasEnum (AI|GetBlackboard 0) (Utilities|Name|MakeLiteralName "AIState") (Utilities|Enum|LiteralenumE_EnemyBheaviorStates "NewEnumerator1")))))

(event EventBeginPlay
  (AI|RunBehaviorTree "/Game/AI_przeciwnicy/BT_frajerzy.BT_frajerzy")
  (bind _asbp_enemy (Utilities|Casting|CastToBP_Enemy (Pawn|GetControlledPawn))
    (:then
      (bind _output_get (Variables|Default|SetEnemy _asbp_enemy))
      (AI|Components|Blackboard|SetValueasEnum (AI|GetBlackboard _output_get) (Utilities|Name|MakeLiteralName "MovementState") (Variables|/Game/AI_przeciwnicy/BP_Enemy.BP_Enemy_C|GetMovementMode _output_get)))
    (:CastFailed
      (Development|PrintString "Fallo el cast"))))

(fn ConstructionScript)