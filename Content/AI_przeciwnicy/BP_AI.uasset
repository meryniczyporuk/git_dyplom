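; Enemy AI character with a revolver that takes damage and, at zero health, ragdolls, stops moving and is flagged dead.
; Fire is blocked when dead and rate-limited by a DoOnce with delayed reset.
; Each shot plays muzzle effects, then line-traces along the mesh's right vector, applying damage, a decal and impact sound without checking for a hit.
; Aim only sets IsAiming; capsule-collision and blackboard-target nodes are left unwired.
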(event Game|Damage|EventAnyDamage
  (params (Damage :type Float%20%28single-precision%29) (DamageType :type Damage%20Type%20Object%20Reference) (InstigatedBy :type Controller%20Object%20Reference) (DamageCauser :type Actor%20Object%20Reference))
  ;[0.5551 1 0.6452] HEALTH SYSTEM
  (Variables|Default|SetHEALTH (- (Variables|Default|GetHEALTH) Damage))
  (if (<= (Variables|Default|GetHEALTH) 0.0)
    (Development|PrintString "CIUPAZECKA")
    (Physics|SetSimulatePhysics (Variables|Character|GetMesh) true)
    (Pawn|Components|CharacterMovement|SetMovementMode (Variables|Character|GetCharacterMovement) "MOVE_None" 0)
    (Variables|Default|SetisDead? true)
    (else
      (Development|PrintString "ŁOSCYOPECEK"))))

(event EventFire
  (bind _rewolwer_ai (Variables|Default|GetRewolwer_AI))
  (bind _mesh (Variables|Character|GetMesh))
  (bind _returnvalue (Transformation|GetWorldRotation _mesh))
  (bind _returnvalue_2 (Transformation|GetSocketTransform _rewolwer_ai "b_gun_muzzleflash" "RTS_World"))
  ;[1 1 1] Fire
  (if (not (Variables|Default|GetisDead?))
    (Utilities|FlowControl|DoOnce false :!label _label
      (:Completed
        (Utilities|FlowControl|Sequence
          (:then_0
            (Effects|SpawnEmitterAttached "/Game/VFX/Inventory/Props/FX/P_Pistol_MuzzleFlash_01.P_Pistol_MuzzleFlash_01" (Variables|Default|GetRewolwer_AI) "b_gun_muzzleflash" (.location _returnvalue_2) _returnvalue "0.250000,0.250000,0.250000" "KeepWorldPosition" true "AutoRelease")
            (Audio|PlaySoundatLocation "/Game/DZWIEK/MS_Pistolero_Fire.MS_Pistolero_Fire" (Transformation|GetActorLocation) "0, 0, 0" 0.35 1.0 0.0 0 0 0 0)
            (bind _outhit (Collision|LineTraceByChannel (.location _returnvalue_2) (+ (.location _returnvalue_2) (* (Math|Vector|GetRightVector _returnvalue) 3e+03)) "TraceTypeQuery1" false 0 "ForDuration"))
            (if true
              (Game|Damage|ApplyDamage (.HitActor (Collision|BreakHitResult _outhit)) 5.0 0 0)
              (Rendering|Decal|SpawnDecalatLocation "/Game/VFX/Inventory/Props/FX/bullet_whole.bullet_whole" (Math|Conversions|ToVector(Float) (Math|Random|RandomIntegerinRange 5 6)) (.ImpactPoint (Collision|BreakHitResult _outhit)) (Math|Rotator|MakeRotfromX (.Normal (Collision|BreakHitResult _outhit))) 8.0)
              (Audio|PlaySoundatLocation "/Game/DZWIEK/MS_bullet.MS_bullet" (.ImpactPoint (Collision|BreakHitResult _outhit)) "0, 0, 0" 0.2 1.0 0.0 0 0 0 0)))
          (:then_1
            (Utilities|FlowControl|Delay 1.0)
            (goto _label Reset)))))))

(event EventAim
  (params (Aim? :type Boolean))
  (Variables|Default|SetisAiming Aim?))

(fn ConstructionScript)