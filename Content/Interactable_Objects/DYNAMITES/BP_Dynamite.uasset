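; BP_Dynamite is a dynamite pickup that the player collects by interacting with it.
; ShowInfo sets a pickup prompt on the HUD, and Interact passes DynamiteValue to BP_Player's ChangeDynamiteAmount, then destroys the actor.
; When that pickup's value is two or more, Interact also creates a tutorial widget and adds it to the viewport.
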(event EventBeginPlay)

(event Collision|EventActorBeginOverlap
  (params (OtherActor :type Actor%20Object%20Reference)))

(event EventTick
  (params (DeltaSeconds :type Float%20%28single-precision%29)))

(event EventShowInfo
  (params (HUD :type WBP%20HUD%20Object%20Reference))
  (Default|SetInfoText HUD "Press [E] to pick up"))

(event EventInteract
  (Default|ChangeDynamiteAmount (.AsBP%20Player (Utilities|Casting|CastToBP_Player (Game|Player|GetPlayerPawn 0))) (Variables|Default|GetDynamiteValue))
  (Actor|DestroyActor)
  (if (>= (Variables|Default|GetDynamiteValue) 2.0)
    (bind _returnvalue (Game|ConstructObjectfromClass (Game|GetPlayerController 0) "/Game/UI/TUTORIAL/Tutorial.TUTORIAL_C"))
    (UserInterface|Viewport|AddtoViewport _returnvalue 0)))

(fn ConstructionScript)